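; Enemy drone that wanders between random reachable points and reports player detection to its AI Blackboard.
; A looping timer line-traces from high above the drone to the player's capsule, caching whether sight is blocked.
; An unblocked player overlap with the Sphere writes the FromSweep flag to IsDetecting.
; Capsule end-overlap clears that key, but tests the overlapped component, not the other actor, against the player.
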(event OnComponentBeginOverlap(Sphere)
  (params (OverlappedComponent :type Primitive%20Component%20Object%20Reference) (OtherActor :type Actor%20Object%20Reference) (OtherComp :type Primitive%20Component%20Object%20Reference) (OtherBodyIndex :type Integer) (bFromSweep :type Boolean) (SweepResult :type Hit%20Result%20Structure%20%28by%20ref%29))
  (bind _output_get (Variables|Default|SetSeePJ (== OtherActor (Variables|Default|GetPlayerRef))))
  (if _output_get
    (if (Variables|Default|GetBlocking%20Hit)
      (Development|PrintString "Bloqueando")
      (else
        (AI|Components|Blackboard|SetValueasBool (AI|GetBlackboard 0) (Utilities|Name|MakeLiteralName "IsDetecting") bFromSweep)))))

(event OnComponentEndOverlap(CapsuleComponent)
  (params (OverlappedComponent :type Primitive%20Component%20Object%20Reference) (OtherActor :type Actor%20Object%20Reference) (OtherComp :type Primitive%20Component%20Object%20Reference) (OtherBodyIndex :type Integer))
  (if (== OverlappedComponent (Variables|Default|GetPlayerRef))
    (AI|Components|Blackboard|SetValueasBool (AI|GetBlackboard 0) (Utilities|Name|MakeLiteralName "IsDetecting") false)))

(event Custom|RandomPoint
  (AI|AIMoveTo self (.RandomLocation (AI|Navigation|GetRandomReachablePointinRadius (Transformation|GetActorLocation) 2.5e+03 0 0)) 0 5.0 false
    (:OnSuccess
      (CallFunction|RandomPoint))))

(event Custom|RayToChar
  (bind _outhit (Collision|LineTraceByChannel (+ (Transformation|GetActorLocation) "0.000000,0.000000,1095.000000") (Transformation|GetWorldLocation (Variables|/Script/Engine.Character|GetCapsuleComponent (Variables|Default|GetPlayerRef))) "TraceTypeQuery1" false 0 "ForOneFrame"))
  (Variables|Default|SetBlocking%20Hit (.bBlockingHit (Collision|BreakHitResult _outhit))))

(event EventBeginPlay
  (bind _returnvalue (Actor|GetActorOfClass "/Game/ThirdPerson/Blueprints/BP_ThirdPersonCharacter.BP_ThirdPersonCharacter_C"))
  (Utilities|IsValid _returnvalue
    (:Is%20Valid
      (Variables|Default|SetPlayerRef _returnvalue)
      (CallFunction|RandomPoint)
      (Utilities|Time|SetTimerbyEvent (delegate Custom|RayToChar) 0.1 true))
    (:Is%20Not%20Valid
      (Development|PrintString "Hello"))))

(fn ConstructionScript)